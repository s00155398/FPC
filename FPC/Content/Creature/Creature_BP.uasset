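; Creature_BP is a creature that turns into a physics ragdoll when shot or stabbed.
; Tagged projectile hits on the mesh apply a bone impulse scaled by the projectile's ImpactMultiplier, then destroy the projectile.
; Stabbed applies a fixed bone impulse and plays an impact sound; both paths disable movement and capsule collision.
; Proximity-based jumping with a randomized cooldown is present but disconnected, and Tick is empty.
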(event OnComponentHit(Mesh)
  (params (HitComponent :type Primitive%20Component%20Object%20Reference) (OtherActor :type Actor%20Object%20Reference) (OtherComp :type Primitive%20Component%20Object%20Reference) (NormalImpulse :type Vector :default "0, 0, 0") (Hit :type Hit%20Result%20Structure%20%28by%20ref%29))
  (if (Math|Boolean|ORBoolean (Actor|ActorHasTag OtherActor "AssaultRifleProjectile") (Actor|ActorHasTag OtherActor "PistolProjectile") (Actor|ActorHasTag OtherActor "ShotgunProjectile") (Actor|ActorHasTag OtherActor "sniper"))
    (bind _asfpcprojectile (Utilities|Casting|CastToFPCProjectile OtherActor))
    (Variables|Default|SetImpact%20Multiplier (Variables|/Script/FPC.FPCProjectile|GetImpactMultiplier _asfpcprojectile))
    (Physics|SetSimulatePhysics (Variables|Character|GetMesh) true)
    (Pawn|Components|CharacterMovement|DisableMovement (Variables|Character|GetCharacterMovement))
    (Class|SkeletalMeshComponent|AddImpulsetoAllBodiesBelow (Variables|Character|GetMesh) (* (Transformation|GetActorForwardVector OtherActor) (Variables|Default|GetImpact%20Multiplier)) (.hitbonename Hit) false true)
    (Variables|Default|SetIsRagdoll true)
    (Collision|SetCollisionEnabled (Variables|Collision|GetCapsuleComponent) "NoCollision")
    (Actor|DestroyActor OtherActor)))

(event Custom|Stabbed
  (params (ForwardVector :type Vector) (BoneName :type Name))
  (Physics|SetSimulatePhysics (Variables|Character|GetMesh) true)
  (Pawn|Components|CharacterMovement|DisableMovement (Variables|Character|GetCharacterMovement))
  (Class|SkeletalMeshComponent|AddImpulsetoAllBodiesBelow (Variables|Character|GetMesh) (* ForwardVector 2e+03) BoneName false true)
  (Variables|Default|SetIsRagdoll true)
  (Collision|SetCollisionEnabled (Variables|Collision|GetCapsuleComponent) "NoCollision")
  (Audio|SpawnSoundatLocation "/Game/FirstPersonCPP/Weapons/Sound/Rifle/Cues/Rifle_ImpactBody_Cue.Rifle_ImpactBody_Cue" (Transformation|GetActorLocation) "0, 0, 0" 1.0 1.0 0.0 0 0))

(event Custom|ResetJump
  (Utilities|FlowControl|Delay (Math|Random|RandomFloatinRange 5.0 1e+01))
  (Variables|Default|SetHasJumped false))

(event EventTick
  (params (DeltaSeconds :type Float%20%28single-precision%29)))

(event EventBeginPlay
  (bind _outactors (Actor|GetAllActorsOfClass "/Game/FirstPersonCPP/Blueprints/FirstPersonCharacter.FirstPersonCharacter_C"))
  (Variables|Default|SetPlayerRef (Utilities|Array|Get(acopy) _outactors)))

(fn ConstructionScript)